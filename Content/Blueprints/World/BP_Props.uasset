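; BP_Props is a world prop Blueprint that can scatter its static mesh around the actor's origin for variation.
; Random Transform, unless Locked is set, gives the mesh a relative location from RandomVectorFromDeviation and a random full-circle yaw.
; That helper holds per-axis random ranges bounded by plus or minus DeviationMax.
; The construction script is empty, so randomization does not run on construction.
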(fn `Random Transform`
  (if (not (`self.Locked`))
    (`SceneComponent.K2_SetRelativeTransform` (`self.StaticMesh`) (`KismetMathLibrary.MakeTransform` (`self.RandomVectorFromDeviation`) (`KismetMathLibrary.MakeRotator` 0.0 0.0 (`KismetMathLibrary.RandomFloatInRange` 0.0 360.0))) false false)))

(fn `UserConstructionScript`)