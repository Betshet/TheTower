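; BP_Rock is a harvestable rock actor that yields resource pickups after enough hits.
; OnHit increments a hit counter and calls Gather once it reaches HitNeeded.
; Gather spawns a configurable number of BP_Ressource actors at the rock's transform, passes each a resource value, then destroys the rock.
; A debug G key triggers OnHit directly.
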(event Input|KeyboardEvents|DebugKeyG
  (params (Key :type Key%20Structure :default "None") (ActionValue :type Input%20Action%20Value%20Structure))
  (:Pressed
    (CallFunction|OnHit)))

(fn ConstructionScript)

(fn Gather
  (for _index (range 0 (- (Variables|Default|GetResourcesSpawn) 1))
    (Game|SpawnActorfromClass "/Game/Blueprints/BP_Ressource.BP_Ressource_C" (Transformation|GetActorTransform) "Undefined" "MultiplyWithRoot" 0 (Variables|Default|GetResourcesValue) 0))
  (Actor|DestroyActor))

(fn OnHit
  (Variables|Default|SetHit (+ (Variables|Default|GetHit) 1))
  (if (>= (Variables|Default|GetHit) (Variables|Default|GetHitNeeded))
    (CallFunction|Gather)))