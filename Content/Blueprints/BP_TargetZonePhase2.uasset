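; Timed hit-zone actor that marks a radius, then kills player characters and triggers hits on rocks inside it when the countdown ends.
; On BeginPlay, outside preview, it sizes a Niagara circle, collision sphere and visual sphere from HitRadius.
; A Timeline matched to the hit delay animates the dynamic material's color, then applies hits to overlapping actors and destroys the zone.
; In preview mode, Tick only updates the collision radius.
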(event `self.ReceiveBeginPlay`
  (bind (_returnvalue_x _returnvalue_y _returnvalue_z) (`KismetMathLibrary.BreakVector` (`self.K2_GetActorLocation`)))
  (bind _timeline (`self.Timeline`))
  (bind _hitradius (`self.HitRadius`))
  (bind _returnvalue (* (`self.HitRadius`) 2.0))
  (bind _returnvalue_2 (/ _hitradius 50.0))
  (if (not (`self.IsPreview`))
    (bind _returnvalue_3 (`NiagaraFunctionLibrary.SpawnSystemAtLocation` "/Game/Art/CIrcle.CIrcle" (`KismetMathLibrary.MakeVector` _returnvalue_x _returnvalue_y (+ _returnvalue_z 0.1))))
    (`NiagaraComponent.SetVariableVec2` _returnvalue_3 "User.CircleSize" (`KismetMathLibrary.MakeVector2D` _returnvalue _returnvalue))
    (`NiagaraComponent.SetVariableFloat` _returnvalue_3 "User.LoopDuration" (`self.DurationBeforeHitInSeconds`))
    (bind _returnvalue_4 (`PrimitiveComponent.CreateDynamicMaterialInstance` (`self.SphereVisual`) 0 "/Game/Art/Materials/SphereCrossSection_Mat.SphereCrossSection_Mat" "None"))
    (bind _output_get (set `self.VisualMaterial` _returnvalue_4))
    (`PrimitiveComponent.SetMaterial` (`self.SphereVisual`) 0 _output_get)
    (`SphereComponent.SetSphereRadius` (`self.Sphere`) _hitradius true)
    (`SceneComponent.SetRelativeScale3D` (`self.SphereVisual`) (`KismetMathLibrary.MakeVector` _returnvalue_2 _returnvalue_2 _returnvalue_2))
    (`TimelineComponent.SetTimelineLength` _timeline (`self.DurationBeforeHitInSeconds`))
    (`TimelineComponent.SetPlayRate` _timeline 1.0)
    (bind (_direction _newtrack_0) (`Timeline|Timeline` :!via `PlayFromStart`)
      (:`Update`
        (`MaterialInstanceDynamic.SetVectorParameterValue` (`self.VisualMaterial`) "Color" _newtrack_0))
      (:`Finished`
        (for _array_element (`PrimitiveComponent.GetOverlappingActors` (`self.Sphere`) "/Script/Engine.Actor")
          (bind _asbp_rock (cast `/Game/Blueprints/BP_Rock` _array_element)
            (:`then`
              (`KismetSystemLibrary.PrintString` "Rock is hit")
              (`/Game/Blueprints/BP_Rock.OnHitEvent` _asbp_rock false))
            (:`CastFailed`
              (bind _asbp_third_person_character (cast `/Game/ThirdPerson/Blueprints/BP_ThirdPersonCharacter` _array_element))
              (`/Game/ThirdPerson/Blueprints/BP_ThirdPersonCharacter.Kill` _asbp_third_person_character))))
        (`self.K2_DestroyActor`)))))

(event `self.ReceiveTick`
  (params (DeltaSeconds :type "Float (single-precision)"))
  (if (`self.IsPreview`)
    (`SphereComponent.SetSphereRadius` (`self.Sphere`) (`self.HitRadius`) true)))

(fn `UserConstructionScript`)