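; BP_ResourceBank is an actor that stores a single resource amount and exposes add, remove, read and collect functions.
; AddResource caps at ResourceMax, but its check re-adds Amount after the update, so it can fill early; RemoveResource floors at zero.
; CollectResources empties the bank and returns the previous amount.
; Changes fire added or removed dispatchers with the new total, with Add and Remove reporting the requested, unclamped amount.
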(fn `AddResource`
  (params (Amount :type Integer))
  (bind _returnvalue (+ Amount (`self.ResourceCurrent`)))
  (set `self.ResourceCurrent` _returnvalue)
  (if (> _returnvalue (`self.ResourceMax`))
    (set `self.ResourceCurrent` (`self.ResourceMax`)))
  (`self.OnRessourceAdded` Amount (`self.ResourceCurrent`)))

(fn `CollectResources`
  (returns (Resources :type Integer))
  (locals (tempRes :type Integer))
  (bind _output_get (set `local.tempRes` (`self.ResourceCurrent`)))
  (set `self.ResourceCurrent` 0)
  (`self.OnRessourceRemoved` _output_get)
  (return _output_get))

(fn `GetCurrentResource`
  (returns (Amount :type Integer))
  (return (`self.ResourceCurrent`)))

(fn `RemoveResource`
  (params (Amount :type Integer))
  (bind _output_get (set `self.ResourceCurrent` (- (`self.ResourceCurrent`) Amount)))
  (if (< _output_get 0)
    (set `self.ResourceCurrent` 0))
  (`self.OnRessourceRemoved` Amount (`self.ResourceCurrent`)))

(fn `UserConstructionScript`)