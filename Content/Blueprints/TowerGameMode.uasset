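; Game mode that bootstraps a tower level, spawning the resource bank, player HUD, moving tower and rock manager on BeginPlay.
; Resource bank add and remove events are forwarded to the HUD.
; The tower spawns at the first BP_TowerSpawner, starting from the waypoint tagged "FirstWaypoint", and rock spawning begins only if that spawner exists.
; ChangePhase stores the new phase, but its switch has no branch logic.
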(event `self.ReceiveBeginPlay`
  (bind _resourcebank (`self.ResourceBank`))
  (bind _returnvalue (`|SpawnActorFromClass` "/Game/Blueprints/BP_ResourceBank.BP_ResourceBank_C" (`KismetMathLibrary.MakeTransform` (0.0 0.0 0.0)) "Undefined" "MultiplyWithRoot" null null))
  (set `self.ResourceBank` _returnvalue)
  (bind _returnvalue_2 (`|CreateWidget` "/Game/UI/WD_PlayerHUD.WD_PlayerHUD_C" (`GameplayStatics.GetPlayerController` 0)))
  (bind _output_get (set `self.PlayerHUD` _returnvalue_2))
  (`UserWidget.AddToViewport` _output_get 0)
  (add `/Game/Blueprints/BP_ResourceBank.OnRessourceAdded` _resourcebank (delegate `OnRessourceAdded_Event`))
  (add `/Game/Blueprints/BP_ResourceBank.OnRessourceRemoved` _resourcebank (delegate `OnRessourceRemoved_Event`))
  (bind _outactors (`GameplayStatics.GetAllActorsOfClass` "/Game/Blueprints/BP_TowerSpawner.BP_TowerSpawner_C"))
  (bind _output (`|GetArrayItem` _outactors))
  (`/Engine/EditorBlueprintResources/StandardMacros.IsValid` _output
    (:`Is Valid`
      (bind _waypoint (`self.FindTowerFirstWaypoint`))
      (bind _returnvalue_3 (`|SpawnActorFromClass` "/Game/Blueprints/BP_MovableTower.BP_MovableTower_C" (`self.GetTransform` _output) "AlwaysSpawn" "MultiplyWithRoot" null _waypoint null))
      (set `self.Tower` _returnvalue_3)
      (bind _returnvalue_4 (`|SpawnActorFromClass` "/Game/Blueprints/BP_RockManager.BP_RockManager_C" (`KismetMathLibrary.MakeTransform` (0.0 0.0 0.0)) "Undefined" "MultiplyWithRoot" null null))
      (`/Game/Blueprints/BP_RockManager.BeginRockSpawnage` _returnvalue_4))))

(event `OnRessourceAdded_Event`
  (params (AmountAdded :type Integer) (CurrentAmount :type Integer))
  (`/Game/UI/WD_PlayerHUD.AddRessource` (`self.PlayerHUD`) AmountAdded CurrentAmount))

(event `OnRessourceRemoved_Event`
  (params (AmountRemoved :type Integer) (CurrentAmount :type Integer))
  (`/Game/UI/WD_PlayerHUD.RemoveRessource` (`self.PlayerHUD`) AmountRemoved CurrentAmount))

(fn `ChangePhase`
  (params (`Old Phase` :type Integer) (`New Phase` :type Integer))
  (set `self.CurrentPhase` `New Phase`)
  (switch `int` `New Phase`))

(fn `FindTowerFirstWaypoint`
  (returns (Waypoint :type "/Game/Blueprints/BP_TowerWaypoint Object Reference"))
  (bind _outactors (`GameplayStatics.GetAllActorsOfClassWithTag` "/Game/Blueprints/BP_TowerWaypoint.BP_TowerWaypoint_C" "FirstWaypoint"))
  (bind _output (`|GetArrayItem` _outactors))
  (`/Engine/EditorBlueprintResources/StandardMacros.IsValid` _output
    (:`Is Valid`
      _)
    (:`Is Not Valid`
      (`KismetSystemLibrary.PrintString` "Failed to find first tower waypoint")))
  (return _output))

(fn `UserConstructionScript`)