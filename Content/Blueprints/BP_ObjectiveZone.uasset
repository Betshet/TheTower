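; BP_ObjectiveZone is a trigger actor that advances the game's objective phase when the player character or a movable tower enters it.
; On overlap, it accepts only BP_MovableTower or BP_ThirdPersonCharacter, then gets the TowerGameMode.
; If the zone's ObjectivePhase matches the game mode's CurrentPhase, it calls ChangePhase to move to its NextPhase, so zones respond only during their assigned phase.
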(event `self.ReceiveActorBeginOverlap`
  (params (OtherActor :type "Actor Object Reference"))
  (cast `/Game/Blueprints/BP_MovableTower` OtherActor
    (:`then`
      _)
    (:`CastFailed`
      (cast `/Game/ThirdPerson/Blueprints/BP_ThirdPersonCharacter` OtherActor)))
  (bind _astower_game_mode (cast `/Game/Blueprints/TowerGameMode` (`GameplayStatics.GetGameMode`)))
  (if (== (`self.Objective Phase`) (`/Game/Blueprints/TowerGameMode.CurrentPhase` _astower_game_mode))
    (`/Game/Blueprints/TowerGameMode.ChangePhase` _astower_game_mode (`self.Objective Phase`) (`self.Next Phase`))))

(fn `UserConstructionScript`)