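; BP_WorldRock is a world rock Blueprint with a routine for randomizing the look of its static mesh.
; Unless Locked, RandomVisual sets a random yaw in 180-degree steps, even with Rotate4Direction on, and a relative location from MaxDeviation via RandomInRange.
; RandomInRange holds only an unconnected symmetric random-float node.
; The construction script is empty, and nothing in the file calls RandomVisual.
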(fn `RandomVisual`
  (bind (_maxdeviation_x _maxdeviation_y _maxdeviation_z) (`KismetMathLibrary.BreakVector` (`self.MaxDeviation`)))
  (if (not (`self.Locked`))
    (if (`self.Rotate 4 Direction`)
      (`SceneComponent.K2_SetRelativeRotation` (`self.StaticMesh`) (`KismetMathLibrary.MakeRotator` 0.0 0.0 (`KismetMathLibrary.Conv_IntToDouble` (* (`KismetMathLibrary.RandomInteger` 4) 180))) false false)
      (else
        (`SceneComponent.K2_SetRelativeRotation` (`self.StaticMesh`) (`KismetMathLibrary.MakeRotator` 0.0 0.0 (`KismetMathLibrary.Conv_IntToDouble` (* (`KismetMathLibrary.RandomInteger` 2) 180))) false false)))
    (`SceneComponent.K2_SetRelativeLocation` (`self.StaticMesh`) (`KismetMathLibrary.MakeVector` (`self.RandomInRange` _maxdeviation_x) (`self.RandomInRange` _maxdeviation_y) (`self.RandomInRange` _maxdeviation_z)) false false)))

(fn `UserConstructionScript`)